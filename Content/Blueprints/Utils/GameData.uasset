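; GameData is a utility set of functions for reaching the ZombieMode game mode's security level and static camera.
; Security level get and set forward to ZombieMode, with the getter returning zero if the cast fails.
; SetStaticCamera stores the camera on ZombieMode and the player's MixamoCharacter_Master and makes it the view target.
; UpdateStaticCamera slowly turns that camera toward the player via VInterpTo, setting pitch and yaw with zero roll.
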(fn GetSecurityLevel
  (bind _aszombie_mode (Utilities|Casting|CastToZombieMode (Game|GetGameMode))
    (:then
      (bind _security_level (CallFunction|GetSecurityLevel _aszombie_mode))
      (return _security_level))
    (:CastFailed
      (return 0))))

(fn SetSecurityLevel
  (params (SecurityLevel :type Integer))
  (bind _aszombie_mode (Utilities|Casting|CastToZombieMode (Game|GetGameMode)))
  (CallFunction|SetSecurityLevel SecurityLevel _aszombie_mode))

(fn SetStaticCamera
  (params (StaticCamera :type Camera%20Actor%20Object%20Reference))
  (LocalVariables|Setl_StaticCamera StaticCamera)
  (bind _aszombie_mode (Utilities|Casting|CastToZombieMode (Game|GetGameMode))
    (:then
      (LocalVariables|SetZombieMode _aszombie_mode)
      (Variables|/Game/Modes/ZombieMode.ZombieMode_C|SetStaticCamera (LocalVariables|GetZombieMode) (LocalVariables|Getl_StaticCamera))
      (Game|Player|SetViewTargetwithBlend (Game|GetPlayerController 0) (LocalVariables|Getl_StaticCamera) 0.0 "VTBlend_Linear" 0.0 false)
      (bind _asmixamo_character_master (Utilities|Casting|CastToMixamoCharacter_Master (Game|GetPlayerCharacter 0))
        (:then
          (Variables|/Game/MixamoAnimPack/MixamoCharacter_Master.MixamoCharacter_Master_C|SetStaticCamera _asmixamo_character_master (Variables|/Game/Modes/ZombieMode.ZombieMode_C|GetStaticCamera (LocalVariables|GetZombieMode)))
          (return))
        (:CastFailed
          (return))))
    (:CastFailed
      (return))))

(fn UpdateStaticCamera
  (params (DeltaT :type Float%20%28single-precision%29))
  (bind _aszombie_mode (Utilities|Casting|CastToZombieMode (Game|GetGameMode)))
  (LocalVariables|Setl_StaticCamera (Variables|/Script/Engine.CameraActor|GetCameraComponent (Variables|/Game/Modes/ZombieMode.ZombieMode_C|GetStaticCamera _aszombie_mode)))
  (LocalVariables|Setl_DeltaT DeltaT)
  (LocalVariables|SetCurrentXVector (Math|Rotator|GetRotationXVector (Transformation|GetWorldRotation (LocalVariables|Getl_StaticCamera))))
  (LocalVariables|SetTargetXVector (- (Transformation|GetActorLocation (Game|GetPlayerCharacter (LocalVariables|Getl_StaticCamera))) (Transformation|GetWorldLocation (LocalVariables|Getl_StaticCamera))))
  (LocalVariables|SetNewYaw (Math|Float|ClampAngle (.yaw (Math|Rotator|MakeRotfromX (Math|Interpolation|VInterpTo (LocalVariables|GetCurrentXVector) (LocalVariables|GetTargetXVector) (LocalVariables|Getl_DeltaT) 0.01))) (- (.yaw (Math|Rotator|MakeRotfromX (Math|Interpolation|VInterpTo (LocalVariables|GetCurrentXVector) (LocalVariables|GetTargetXVector) (LocalVariables|Getl_DeltaT) 0.01))) (LocalVariables|GetInterpSpeed)) (+ (.yaw (Math|Rotator|MakeRotfromX (Math|Interpolation|VInterpTo (LocalVariables|GetCurrentXVector) (LocalVariables|GetTargetXVector) (LocalVariables|Getl_DeltaT) 0.01))) (LocalVariables|GetInterpSpeed))))
  (LocalVariables|SetNewPitch (Math|Float|ClampAngle (.pitch (Math|Rotator|MakeRotfromX (Math|Interpolation|VInterpTo (LocalVariables|GetCurrentXVector) (LocalVariables|GetTargetXVector) (LocalVariables|Getl_DeltaT) 0.01))) (- (.pitch (Math|Rotator|MakeRotfromX (Math|Interpolation|VInterpTo (LocalVariables|GetCurrentXVector) (LocalVariables|GetTargetXVector) (LocalVariables|Getl_DeltaT) 0.01))) (LocalVariables|GetInterpSpeed)) (+ (.pitch (Math|Rotator|MakeRotfromX (Math|Interpolation|VInterpTo (LocalVariables|GetCurrentXVector) (LocalVariables|GetTargetXVector) (LocalVariables|Getl_DeltaT) 0.01))) (LocalVariables|GetInterpSpeed))))
  (Transformation|SetWorldRotation (LocalVariables|Getl_StaticCamera) (Math|Rotator|MakeRotator 0.0 (LocalVariables|GetNewPitch) (LocalVariables|GetNewYaw)) false false))