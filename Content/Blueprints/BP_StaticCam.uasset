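; BP_StaticCam is a static camera actor that calls SetStaticCamera on itself when the player character enters its trigger volume.
; An overlap of the Box by a MixamoCharacter_Master triggers the switch, as does BeginPlay when InitialCamera is set.
; The construction script sizes and positions the Box from the Extent and Location variables.
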(event `self.ReceiveBeginPlay`
  (if (`self.Initial Camera`)
    (`/Game/Blueprints/Utils/GameData.SetStaticCamera` self)))

(event `self.ReceiveActorBeginOverlap`
  (params (OtherActor :type "Actor Object Reference")))

(event `self.ReceiveTick`
  (params (DeltaSeconds :type "Float (single-precision)")))

(event `self.Box.OnComponentBeginOverlap`
  (params (OtherActor :type "Actor Object Reference") (OtherComp :type "PrimitiveComponent Object Reference") (OtherBodyIndex :type Integer) (bFromSweep :type Boolean) (SweepResult :type "HitResult Structure (by ref)"))
  (cast `/Game/MixamoAnimPack/MixamoCharacter_Master` OtherActor)
  (`/Game/Blueprints/Utils/GameData.SetStaticCamera` self))

(fn `UserConstructionScript`
  (`BoxComponent.SetBoxExtent` (`self.Box`) (`self.Extent`) true)
  (`SceneComponent.K2_SetRelativeLocation` (`self.Box`) (`self.Location`) false false))