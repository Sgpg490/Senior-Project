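; Door Blueprint that the player opens and closes with the U key while near it.
; TriggerBox overlap begin and end enable and disable input for player controller 0, without checking which actor overlaps.
; Each press flips DoorStatus and plays or reverses the DoorMovement timeline.
; The timeline lerps the relative location of TriggerBox itself between DoorStart and DoorEnd, so the trigger volume moves during the motion.
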(event `self.TriggerBox.OnComponentBeginOverlap`
  (params (OtherActor :type "Actor Object Reference") (OtherComp :type "PrimitiveComponent Object Reference") (OtherBodyIndex :type Integer) (bFromSweep :type Boolean) (SweepResult :type "HitResult Structure (by ref)"))
  (`self.EnableInput` (`GameplayStatics.GetPlayerController` 0)))

(event `self.TriggerBox.OnComponentEndOverlap`
  (params (OtherActor :type "Actor Object Reference") (OtherComp :type "PrimitiveComponent Object Reference") (OtherBodyIndex :type Integer))
  (`self.DisableInput` (`GameplayStatics.GetPlayerController` 0)))

(event `Key|U`
  (params (Key :type "Key Structure" :default "AnyKey"))
  (:`Pressed`
    (if (`self.DoorStatus`)
      (set `self.DoorStatus` false)
      (bind (_direction _doormove) (`Timeline|DoorMovement` :!label _label)
        (:`Update`
          (`SceneComponent.K2_SetRelativeLocation` (`self.TriggerBox`) (`KismetMathLibrary.VLerp` (`self.DoorStart`) (`self.Door End`) _doormove) false false)))
      (else
        (set `self.DoorStatus` true)
        (goto _label :!via `Reverse`)))))

(fn `UserConstructionScript`)